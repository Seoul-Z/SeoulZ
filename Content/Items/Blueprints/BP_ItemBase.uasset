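; BP_ItemBase is an item actor Blueprint that gets its name and mesh from a data table.
; GetItemData looks up the row referenced by the ItemDataComp row handle.
; OnLookAt formats that row's name into a "PickUp {Item}" prompt, and SetItemSKM applies its static mesh to StaticMesh.
; The event graph and construction script are empty; only the default-named 새 함수 calls SetItemSKM here.
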(event EventBeginPlay)

(event Collision|EventActorBeginOverlap
  (params (OtherActor :type Actor%20Object%20Reference)))

(event EventTick
  (params (DeltaSeconds :type Float%20%28single-precision%29)))

(fn ConstructionScript)

(fn GetItemData
  (bind _itemdatacomp (Variables|Default|GetItemDataComp))
  (bind _itemrowhandle (Variables|/Script/ProjectSeoulZ.SZItemDataComp|GetItemRowHandle _itemdatacomp))
  (bind _returnvalue (Utilities|GetDataTableRow (.datatable _itemrowhandle) (.rowname _itemrowhandle))
    (:then
      (return _returnvalue))))

(fn OnLookat
  (return (Utilities|Text|FormatText "PickUp {Item}" (.Name (Utilities|Struct|BreakS_ItemDefinition (CallFunction|GetItemData))))))

(fn SetItemSKM
  (Components|StaticMesh|SetStaticMesh (Variables|Default|GetStaticMesh) (.StaticMesh (Utilities|Struct|BreakS_ItemMesh (.Mesh (Utilities|Struct|BreakS_ItemDefinition (CallFunction|GetItemData)))))))

(fn 새함수
  (CallFunction|SetItemSKM))